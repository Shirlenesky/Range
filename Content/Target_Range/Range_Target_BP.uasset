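; Shooting range target that slides back and forth and awards points to the player when FirstPersonProjectile hits it.
; Two chained timelines lerp it between its start position and a fixed Y, looping endlessly.
; Head and Body overlaps add different points to the FirstPersonCharacter, each with its own sound.
; The high score loads from a SaveGameHS slot at BeginPlay and is saved whenever points match or beat it.
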(event `self.ReceiveBeginPlay`
  (bind (_returnvalue_x _returnvalue_y _returnvalue_z) (`KismetMathLibrary.BreakVector` (`self.K2_GetActorLocation`)))
  (bind _slot_name (`self.slot Name`))
  (set `self.Start` (`KismetMathLibrary.MakeVector` _returnvalue_x _returnvalue_y _returnvalue_z))
  (set `self.End` (`KismetMathLibrary.MakeVector` _returnvalue_x -1700.0 _returnvalue_z))
  (bind _asfirst_person_character (cast `/Game/FirstPersonBP/Blueprints/FirstPersonCharacter` (`GameplayStatics.GetPlayerCharacter` 0)))
  (set `self.Char REF` _asfirst_person_character)
  (bind _returnvalue (`GameplayStatics.DoesSaveGameExist` _slot_name))
  (if _returnvalue
    (bind _returnvalue_2 (`GameplayStatics.LoadGameFromSlot` _slot_name))
    (bind _output_get (set `self.SaverSubClass` _returnvalue_2))
    (bind _assave_game_hs (cast `/Game/FirstPersonBP/Blueprints/SaveGameHS` _output_get))
    (set `/Game/FirstPersonBP/Blueprints/FirstPersonCharacter.HighScore` (`/Game/FirstPersonBP/Blueprints/SaveGameHS.High Score` _assave_game_hs) (`self.Char REF`))
    (bind (_direction _move) (`Timeline|Move` :!via `PlayFromStart` :!label _label)
      (:`Update`
        (`self.K2_SetActorRelativeLocation` (`KismetMathLibrary.VLerp` (`self.Start`) (`self.End`) _move)))
      (:`Finished`
        (bind (_direction_2 _move_2) (`Timeline|Move Back` :!via `ReverseFromEnd`)
          (:`Update`
            (`self.K2_SetActorRelativeLocation` (`KismetMathLibrary.VLerp` (`self.Start`) (`self.End`) _move_2)))
          (:`Finished`
            (goto _label :!via `PlayFromStart`)))))
    (else
      (goto _label :!via `PlayFromStart`))))

(event `self.Head.OnComponentBeginOverlap`
  (params (OverlappedComponent :type "PrimitiveComponent Object Reference") (OtherActor :type "Actor Object Reference") (OtherComp :type "PrimitiveComponent Object Reference") (OtherBodyIndex :type Integer) (bFromSweep :type Boolean) (SweepResult :type "HitResult Structure (by ref)"))
  (bind _slot_name (`self.slot Name`))
  (bind _saversubclass (`self.SaverSubClass`))
  (bind _char_ref (`self.Char REF`))
  (bind _points (`/Game/FirstPersonBP/Blueprints/FirstPersonCharacter.Points` _char_ref))
  (cast `/Game/FirstPersonBP/Blueprints/FirstPersonProjectile` OtherActor)
  (set `/Game/FirstPersonBP/Blueprints/FirstPersonCharacter.Points` (+ _points 10) _char_ref)
  (`GameplayStatics.PlaySoundAtLocation` "/Game/Target_Range/bui.bui" (`self.K2_GetActorLocation`) (struct) 1.0 1.0 0.0 null null null)
  (if (>= _points (`/Game/FirstPersonBP/Blueprints/FirstPersonCharacter.HighScore` _char_ref)) :!label _label_2
    (bind _output_get (set `/Game/FirstPersonBP/Blueprints/FirstPersonCharacter.HighScore` _points _char_ref))
    (bind _returnvalue (`GameplayStatics.DoesSaveGameExist` (`self.slot Name`)))
    (if _returnvalue
      (bind _returnvalue_2 (`GameplayStatics.LoadGameFromSlot` (`self.slot Name`)))
      (bind _output_get_2 (set `self.SaverSubClass` _returnvalue_2))
      (bind _assave_game_hs (cast `/Game/FirstPersonBP/Blueprints/SaveGameHS` _output_get_2))
      (set `/Game/FirstPersonBP/Blueprints/SaveGameHS.High Score` _output_get _assave_game_hs)
      (`GameplayStatics.SaveGameToSlot` _saversubclass _slot_name)
      (else
        (bind _returnvalue_3 (`GameplayStatics.CreateSaveGameObject` "/Game/FirstPersonBP/Blueprints/SaveGameHS.SaveGameHS_C"))
        (bind _output_get_3 (set `self.SaverSubClass` _returnvalue_3))
        (bind _assave_game_hs_2 (cast `/Game/FirstPersonBP/Blueprints/SaveGameHS` _output_get_3))
        (set `/Game/FirstPersonBP/Blueprints/SaveGameHS.High Score` _output_get _assave_game_hs_2)
        (`GameplayStatics.SaveGameToSlot` _saversubclass _slot_name)))))

(event `self.Body.OnComponentBeginOverlap`
  (params (OverlappedComponent :type "PrimitiveComponent Object Reference") (OtherActor :type "Actor Object Reference") (OtherComp :type "PrimitiveComponent Object Reference") (OtherBodyIndex :type Integer) (bFromSweep :type Boolean) (SweepResult :type "HitResult Structure (by ref)"))
  (bind _char_ref (`self.Char REF`))
  (cast `/Game/FirstPersonBP/Blueprints/FirstPersonProjectile` OtherActor)
  (set `/Game/FirstPersonBP/Blueprints/FirstPersonCharacter.Points` (+ (`/Game/FirstPersonBP/Blueprints/FirstPersonCharacter.Points` _char_ref) 5) _char_ref)
  (`GameplayStatics.PlaySoundAtLocation` "/Game/Target_Range/pu.pu" (`self.K2_GetActorLocation`) (struct) 1.0 1.0 0.0 null null null)
  (goto _label_2))

(fn `UserConstructionScript`)